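; Checkpoint actor that registers itself as the player's last saved position when reached.
; Overlapping its collision with an actor that casts to PlayerController triggers ActiveCheckpoint.
; That function sets the checkpoint-activated flag and passes the checkpoint itself as LastPosition to PlayerGameMode through public setters.
; It then hides the actor and disables that collision, making it single-use.
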(event `self.CheckpointCollision.OnComponentBeginOverlap`
  (params (OverlappedComponent :type "PrimitiveComponent Object Reference") (OtherActor :type "Actor Object Reference") (OtherComp :type "PrimitiveComponent Object Reference") (OtherBodyIndex :type Integer) (bFromSweep :type Boolean) (SweepResult :type "HitResult Structure (by ref)"))
  ;[1 1 1] Activamos Checkpoint cuando el Player choque con la colision
  (cast `/Game/Blueprints/Player/Blueprints/Player/PlayerController` OtherActor)
  (`self.ActiveCheckpoint`))

(fn `ActiveCheckpoint`
  ;[1 1 1] Hacemos cast del game mode y seteamos la variable privada IsCheckpointActived mediante una función pública.
  (bind _asbp_first_person_game_mode (cast `/Game/Blueprints/Player/GameMode/PlayerGameMode` (`GameplayStatics.GetGameMode`)))
  (`/Game/Blueprints/Player/GameMode/PlayerGameMode.SetIsCheckpointActived` _asbp_first_person_game_mode true)
  ;[1 1 1] Del game mode, mediante una función set, seteamos la variable privada LastPosition con la referencia de este mismo actor, de esta forma guardamos la posición del propio checkpoint.
  (`/Game/Blueprints/Player/GameMode/PlayerGameMode.SetLastPosition` _asbp_first_person_game_mode self)
  ;[1 1 1] Para finalizar escondemos el actor para que no lo podamos ver y desactivamos las colisiones.
  (`self.SetActorHiddenInGame` true)
  (`PrimitiveComponent.SetCollisionEnabled` (`self.CheckpointCollision`) "NoCollision"))

(fn `UserConstructionScript`)