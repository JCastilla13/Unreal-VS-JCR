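; NextLevelCheck is a level-exit trigger that advances the game through its fixed sequence of levels.
; When an actor that casts to PlayerController begins overlapping the CheckWin collision, it deletes the save slot so the pumpkin count restarts.
; NextLevel then compares the current level name to open the following one, from Tutorial through Mid to Extreme, and finally back to the main menu.
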(event `self.CheckWin.OnComponentBeginOverlap`
  (params (OverlappedComponent :type "PrimitiveComponent Object Reference") (OtherActor :type "Actor Object Reference") (OtherComp :type "PrimitiveComponent Object Reference") (OtherBodyIndex :type Integer) (bFromSweep :type Boolean) (SweepResult :type "HitResult Structure (by ref)"))
  ;[1 1 1] Cuando el personaje choque con la colisión de CheckWin se borrará el save actual para poder reiniciar el número de calabazas en el siguiente nivel.
  (cast `/Game/Blueprints/Player/Blueprints/Player/PlayerController` OtherActor)
  (`GameplayStatics.DeleteGameInSlot` (`self.SaveFile`))
  ;[1 1 1] Esta es la función que se encarga de enviarnos al siguiente nivel.
  (`self.NextLevel`))

(fn `NextLevel`
  ;[1 1 1] En esta función lo primero que hacemos es revisar en que nivel estamos y dependiendo de la respuesta el CheckWin nos enviará a un nivel u otro.
  (bind _returnvalue (`GameplayStatics.GetCurrentLevelName` true))
  (`|ExecutionSequence`
    (:`then_0`
      (if (`KismetStringLibrary.EqualEqual_StrStr` _returnvalue (`self.TutorialLevel`))
        (`GameplayStatics.OpenLevelBySoftObjectPtr` "/Game/Levels/MidLevel.MidLevel")))
    (:`then_1`
      (if (`KismetStringLibrary.EqualEqual_StrStr` _returnvalue (`self.MidLevel`))
        (`GameplayStatics.OpenLevelBySoftObjectPtr` "/Game/Levels/ExtremeLevel.ExtremeLevel")))
    (:`then_2`
      (if (`KismetStringLibrary.EqualEqual_StrStr` _returnvalue (`self.ExtremeLevel`))
        (`GameplayStatics.OpenLevelBySoftObjectPtr` "/Game/Levels/MainMenu.MainMenu")))))

(fn `UserConstructionScript`)