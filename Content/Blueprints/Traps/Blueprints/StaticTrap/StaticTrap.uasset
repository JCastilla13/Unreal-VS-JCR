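; StaticTrap is a static hazard that saves the player's pumpkin count and respawns the player on contact.
; When its collision overlaps a PlayerController, it copies the current pumpkin quantity into that player's PumpkinSaves object and writes it to a save slot.
; It then delegates the respawn to PlayerGameMode through CheckRespawnPlayer.
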(event `self.StaticTrapCollision.OnComponentBeginOverlap`
  (params (OverlappedComponent :type "PrimitiveComponent Object Reference") (OtherActor :type "Actor Object Reference") (OtherComp :type "PrimitiveComponent Object Reference") (OtherBodyIndex :type Integer) (bFromSweep :type Boolean) (SweepResult :type "HitResult Structure (by ref)"))
  ;[1 1 1] Cuando el Player colisione con la trampa, cogemos la variable privada RefPumpkinSave mediante una función Get para llamar a los nodos que se encargarán de guardar la cantidad de calabazas actuales.
  (bind _asplayer_controller (cast `/Game/Blueprints/Player/Blueprints/Player/PlayerController` OtherActor))
  (bind _refpumpkinsave (`/Game/Blueprints/Player/Blueprints/Player/PlayerController.GetRefPumpkinSave` _asplayer_controller))
  ;[1 1 1] Mediante la función Get de PlayerPumpkinQuantity cogemos las calabazas actuales y con un cast a PumpkinSaves le añadimos las calabazas actuales a la función Set que contiene la variable PumpkinQuantitySaves. Después hacemos un save en el archivo que almacena la cantidad de calabazas que tiene el Player en el propio nivel.
  (bind _getquantity (`/Game/Blueprints/Player/Blueprints/Player/PlayerController.GetPlayerPumpkinQuantity` _asplayer_controller))
  (bind _aspumpkin_saves (cast `/Game/Blueprints/Saves/Blueprints/PumpkinSaves/PumpkinSaves` _refpumpkinsave))
  (`/Game/Blueprints/Saves/Blueprints/PumpkinSaves/PumpkinSaves.SetPumpkinQuantitySave` _aspumpkin_saves _getquantity)
  (`GameplayStatics.SaveGameToSlot` _refpumpkinsave (`self.SaveFile`))
  ;[1 1 1] Función que respawnea al Player.
  (`self.RespawnPlayer`))

(fn `RespawnPlayer`
  ;[1 1 1] Hacemos un cast al game mode y llamamos a la función Respawn Player que se encarga de spawnear al Player en las diferentes posiciones disponibles.
  (bind _asplayer_game_mode (cast `/Game/Blueprints/Player/GameMode/PlayerGameMode` (`GameplayStatics.GetGameMode`)))
  (`/Game/Blueprints/Player/GameMode/PlayerGameMode.CheckRespawnPlayer` _asplayer_game_mode))

(fn `UserConstructionScript`)