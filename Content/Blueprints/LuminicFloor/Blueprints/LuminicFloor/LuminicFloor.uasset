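; LuminicFloor is a floor Blueprint that is revealed by contact with the Pumpkin actor.
; When a Pumpkin begins overlapping LuminicCollision, the floor component becomes visible.
; When the overlap ends, a custom event waits TimeFloorVisible seconds, then hides it, and re-entry does not cancel that pending hide.
; Only visibility is toggled, without propagating to child components.
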(event `self.LuminicCollision.OnComponentBeginOverlap`
  (params (OverlappedComponent :type "PrimitiveComponent Object Reference") (OtherActor :type "Actor Object Reference") (OtherComp :type "PrimitiveComponent Object Reference") (OtherBodyIndex :type Integer) (bFromSweep :type Boolean) (SweepResult :type "HitResult Structure (by ref)"))
  ;[1 1 1] Cuando la calabaza colisione con el LuminicFloor este se hará visible.
  (cast `/Game/Blueprints/Pumpkin/Blueprints/Pumpkin/Pumpkin` OtherActor)
  (`self.LuminicFloorVisible`))

(event `self.LuminicCollision.OnComponentEndOverlap`
  (params (OverlappedComponent :type "PrimitiveComponent Object Reference") (OtherActor :type "Actor Object Reference") (OtherComp :type "PrimitiveComponent Object Reference") (OtherBodyIndex :type Integer))
  ;[1 1 1] Cuando deje de colisionar con la calabaza se hará el Event Custom LuminicFloorHidden.
  (cast `/Game/Blueprints/Pumpkin/Blueprints/Pumpkin/Pumpkin` OtherActor)
  (`self.LuminicFloorHidden`))

(event `LuminicFloorHidden`
  ;[1 1 1] Custom Event que esconde los suelos lumínicos tras pasar 5 segundos.
  (`KismetSystemLibrary.Delay` (`self.TimeFloorVisible`))
  (`SceneComponent.SetVisibility` (`self.LuminicFloor`) false false))

(fn `LuminicFloorVisible`
  ;[1 1 1] Hacemos visible el LuminicFloor
  (`SceneComponent.SetVisibility` (`self.LuminicFloor`) true false))

(fn `UserConstructionScript`)