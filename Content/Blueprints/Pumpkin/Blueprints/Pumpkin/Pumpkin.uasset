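; Pumpkin projectile thrown by the player, with speed and launch sound that depend on the throw's charge level.
; Every Tick, it finds the PlayerController via GetActorOfClass and polls its four charge flags to set ProjectileMovement's InitialSpeed and MaxSpeed to the low, mid, high or extreme value.
; On BeginPlay it plays a normal or extreme throw sound, clearing the player's extreme-charge flag in the latter case.
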(event `self.ReceiveTick`
  (params (DeltaSeconds :type "Float (single-precision)"))
  ;[1 1 1] Dentro del event tick comprobamos todo el rato la fuerza con la que lanzamos la calabaza.
  (`self.ChangePumpkinSpeed`))

(event `self.ReceiveBeginPlay`
  ;[1 1 1] Al momento de spawnear la calabaza se escuchará un sonido determinado.
  (`self.PlayDiffSounds`))

(fn `ChangePumpkinSpeed`
  ;[1 1 1] Cogemos referencia del Player utilizando el nodo Get Actor Of Class y mediante un Sequence revisamos con funciones get, las variables booleanas privadas del Player que definen con que fuerza se deben tirar las calabazas.
  (bind _returnvalue (`GameplayStatics.GetActorOfClass` "/Game/Blueprints/Player/Blueprints/Player/PlayerController.PlayerController_C"))
  (`|ExecutionSequence`
    (:`then_0`
      (bind _getlowcharge (`/Game/Blueprints/Player/Blueprints/Player/PlayerController.GetIsLowCharged` _returnvalue)))
    (:`then_1`
      (bind _getmidcharge (`/Game/Blueprints/Player/Blueprints/Player/PlayerController.GetIsMidCharged` _returnvalue)))
    (:`then_2`
      (bind _gethightcharge (`/Game/Blueprints/Player/Blueprints/Player/PlayerController.GetIsHightCharged` _returnvalue)))
    (:`then_3`
      (bind _getextremecharge (`/Game/Blueprints/Player/Blueprints/Player/PlayerController.Get Is Extreme Charged` _returnvalue))))
  ;[1 1 1] Según la variable bool que haya tocado hará una determinada función que determinará la fuerza con la que se lanza la calabaza.
  (`|ExecutionSequence`
    (:`then_0`
      (if _getlowcharge
        (`self.LowSpeed`)))
    (:`then_1`
      (if _getmidcharge
        (`self.MidSpeed`)))
    (:`then_2`
      (if _gethightcharge
        (`self.HightSpeed`)))
    (:`then_3`
      (if _getextremecharge
        (`self.ExtremeSpeed`)))))

(fn `ExtremeSpeed`
  (bind _projectilemovement (`self.ProjectileMovement`))
  ;[1 1 1] Seteamos la velocidad a la que se lanzará la calabaza. En este caso velocidad Extreme.
  (`|ExecutionSequence`
    (:`then_0`
      (set `ProjectileMovementComponent.InitialSpeed` (`self.ExtremeSpeedValue`) _projectilemovement))
    (:`then_1`
      (set `ProjectileMovementComponent.MaxSpeed` (`self.ExtremeSpeedValue`) _projectilemovement))))

(fn `HightSpeed`
  (bind _projectilemovement (`self.ProjectileMovement`))
  ;[1 1 1] Seteamos la velocidad a la que se lanzará la calabaza. En este caso velocidad Hight.
  (`|ExecutionSequence`
    (:`then_0`
      (set `ProjectileMovementComponent.InitialSpeed` (`self.HightSpeedValue`) _projectilemovement))
    (:`then_1`
      (set `ProjectileMovementComponent.MaxSpeed` (`self.HightSpeedValue`) _projectilemovement))))

(fn `LowSpeed`
  (bind _projectilemovement (`self.ProjectileMovement`))
  ;[1 1 1] Seteamos la velocidad a la que se lanzará la calabaza. En este caso velocidad Low.
  (`|ExecutionSequence`
    (:`then_0`
      (set `ProjectileMovementComponent.InitialSpeed` (`self.LowSpeedValue`) _projectilemovement))
    (:`then_1`
      (set `ProjectileMovementComponent.MaxSpeed` (`self.LowSpeedValue`) _projectilemovement))))

(fn `MidSpeed`
  (bind _projectilemovement (`self.ProjectileMovement`))
  ;[1 1 1] Seteamos la velocidad a la que se lanzará la calabaza. En este caso velocidad Mid.
  (`|ExecutionSequence`
    (:`then_0`
      (set `ProjectileMovementComponent.InitialSpeed` (`self.MidSpeedValue`) _projectilemovement))
    (:`then_1`
      (set `ProjectileMovementComponent.MaxSpeed` (`self.MidSpeedValue`) _projectilemovement))))

(fn `PlayDiffSounds`
  ;[1 1 1] Esta función hace una referencia al Player para revisar si lanza la calabaza con la fuerza extrema o no. Si esto es falso, al spawnear la calabaza hará un tipo de sonido, pero si es verdadero, al spawnear la calabaza hará un tipo distinto de sonido y seteará la variable IsExtremeCharged como false.
  (bind _returnvalue (`GameplayStatics.GetActorOfClass` "/Game/Blueprints/Player/Blueprints/Player/PlayerController.PlayerController_C"))
  (bind _getextremecharge (`/Game/Blueprints/Player/Blueprints/Player/PlayerController.Get Is Extreme Charged` _returnvalue))
  (if _getextremecharge
    (`AudioComponent.Play` (`self.SpacialThrowExtremePumpkin`) 0.0)
    (`/Game/Blueprints/Player/Blueprints/Player/PlayerController.SetIsExtremeCharged` _returnvalue false)
    (else
      (`AudioComponent.Play` (`self.SpacialThrowPumpkin`) 0.0))))

(fn `UserConstructionScript`)